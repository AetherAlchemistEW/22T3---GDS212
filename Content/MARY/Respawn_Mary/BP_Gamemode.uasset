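; Game mode that respawns the Neon Dash third-person swapper character and opens the pause menu.
; On begin play and each respawn it enables its own input, applies the camera boom length and binds to the character's destruction.
; When destroyed, a replacement spawns at a stored transform after a short delay and is possessed by the controller saved at PostLogin.
; The pause input shows the cursor, pauses the game and adds the menu widget.
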(event `self.ReceiveBeginPlay`
  ;[1 1 1] Begin event
  (bind _asbp_def_third_person_swapper_neon_dash (cast `/Game/Default_Controls/Blueprints/BP_DEF_ThirdPerson_Swapper_NeonDash` (`GameplayStatics.GetPlayerCharacter` 0) :!label _label))
  (`self.EnableInput` (`GameplayStatics.GetPlayerController` 0))
  (set `/Game/Default_Controls/Blueprints/BP_DEF_ThirdPerson_Swapper_NeonDash.CameraBoomLength` (`self.Camera Boom Length`) _asbp_def_third_person_swapper_neon_dash)
  (add `self.OnDestroyed` _asbp_def_third_person_swapper_neon_dash (delegate `OnDestroyed_Event_0`)))

(event `Respawn`
  ;[1 1 1] Begin event
  (goto _label))

(event `InputAction|PauseGame`
  (params (Key :type "Key Structure"))
  ;[1 1 1] PauseMenu
  (:`Pressed`
    (`KismetSystemLibrary.PrintString` "Pausing")
    (set `PlayerController.bShowMouseCursor` true (`GameplayStatics.GetPlayerController` 0))
    (`GameplayStatics.SetGamePaused` true)
    (bind _returnvalue (`|CreateWidget` "/Game/PauseMenu.PauseMenu_C"))
    (`UserWidget.AddToViewport` _returnvalue 0)))

(event `OnDestroyed_Event_0` :!signature `self.OnDestroyed`
  (params (DestroyedActor :type "Actor Object Reference"))
  ;[1 1 1] Respawn
  (`KismetSystemLibrary.Delay` 0.2)
  (bind _returnvalue (`|SpawnActorFromClass` "/Game/Default_Controls/Blueprints/BP_DEF_ThirdPerson_Swapper_NeonDash.BP_DEF_ThirdPerson_Swapper_NeonDash_C" (`self.Spawn Transform`) "Undefined" "OverrideRootScale" null null))
  (`Controller.Possess` (`self.ControllerRef`) _returnvalue)
  (`self.Respawn`))

(event `self.K2_PostLogin`
  (params (NewPlayer :type "PlayerController Object Reference"))
  ;[1 1 1] Respawn
  (bind _output_get (set `self.ControllerRef` NewPlayer))
  (`self.RestartPlayer` _output_get))

(fn `UserConstructionScript`)